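; Actor component that stores base and current character stats in maps, such as Health and Stamina.
; Changes through SetCurrentStatValue broadcast an update event; ModifyCurrentStartValue clamps to the base value and can trigger regen.
; Stamina regen waits on a retriggerable delay, then a looping timer refills it to MaxValue.
; TakeDamage writes Health directly, skipping the broadcast, and changes the owner's StateManagerComponent state at zero; BeginPlay sets Health to zero.
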(event `self.ReceiveBeginPlay`
  (`self.SetCurrentStatValue` "NewEnumerator1"))

(event `StartRegen`
  (params (StartType :type "/Game/SoulsDeMujerts/Blueprints/Enums/E_Stats Enum" :default "NewEnumerator0"))
  (switch `/Game/SoulsDeMujerts/Blueprints/Enums/E_Stats` StartType
    (:`NewEnumerator2`
      (`KismetSystemLibrary.K2_ClearTimer` null "RegenStamina")
      (`KismetSystemLibrary.RetriggerableDelay` 1.5)
      (`KismetSystemLibrary.K2_SetTimer` null "RegenStamina" 0.1 true))))

(fn `Get Current Start Value`
  (params (Stat :type "/Game/SoulsDeMujerts/Blueprints/Enums/E_Stats Enum" :default "NewEnumerator0"))
  (returns (Value :type "Float (double-precision)"))
  (return (`BlueprintMapLibrary.Map_Find` (`self.CurrentStats`) Stat)))

(fn `GetBaseSartValue`
  (params (Start :type "/Game/SoulsDeMujerts/Blueprints/Enums/E_Stats Enum" :default "NewEnumerator0"))
  (returns (`Base Value` :type "Float (double-precision)"))
  (return (break `/Game/SoulsDeMujerts/Blueprints/Structs/F_BaseStat` (`BlueprintMapLibrary.Map_Find` (`self.BaseStats`) Start))))

(fn `GetMaxValue`
  (params (Start :type "/Game/SoulsDeMujerts/Blueprints/Enums/E_Stats Enum" :default "NewEnumerator0"))
  (returns (Value :type "Float (double-precision)"))
  (return (`.MaxValue_4_7F922FEB4DD93BF935646CAB36125B2D` (break `/Game/SoulsDeMujerts/Blueprints/Structs/F_BaseStat` (`BlueprintMapLibrary.Map_Find` (`self.BaseStats`) Start)))))

(fn `InitializeStats`
  (bind _keys (`BlueprintMapLibrary.Map_Keys` (`self.BaseStats`)))
  (for _array_element _keys
    (`self.SetCurrentStatValue` _array_element (break `/Game/SoulsDeMujerts/Blueprints/Structs/F_BaseStat` (`BlueprintMapLibrary.Map_Find` (`self.BaseStats`) _array_element)))))

(fn `ModifyCurrentStartValue`
  (params (Stat :type "/Game/SoulsDeMujerts/Blueprints/Enums/E_Stats Enum" :default "NewEnumerator0") (Value :type "Float (double-precision)") (`bShouldRegenerate?` :type Boolean :default true))
  (locals (l_Value :type "Float (double-precision)"))
  (if (!= Value 0.0)
    (bind _output_get (set `local.l_Value` (+ (`self.Get Current Start Value` (`local.Stat`)) (`local.Value`))))
    (bind _output_get_2 (set `local.l_Value` (`KismetMathLibrary.FClamp` _output_get 0.0 (`self.GetBaseSartValue` (`local.Stat`)))))
    (`self.SetCurrentStatValue` (`local.Stat`) _output_get_2)
    (if (`local.bShouldRegenerate?`)
      (`self.StartRegen` (`local.Stat`)))))

(fn `RegenStamina`
  (`self.SetCurrentStatValue` "NewEnumerator2" (`KismetMathLibrary.FClamp` (+ (`self.Get Current Start Value` "NewEnumerator2") (`self.StaminaRegenRate`)) 0.0 (`self.GetMaxValue` "NewEnumerator2")))
  (if (>= (`self.Get Current Start Value` "NewEnumerator2") (`self.GetMaxValue` "NewEnumerator2"))
    (`KismetSystemLibrary.K2_ClearTimer` null "RegenStamina")))

(fn `SetBaseStatValue`
  (params (Start :type "/Game/SoulsDeMujerts/Blueprints/Enums/E_Stats Enum" :default "NewEnumerator0") (Value :type "Float (double-precision)"))
  (bind _structout (setmembers `/Game/SoulsDeMujerts/Blueprints/Structs/F_BaseStat` :`StructRef` (`BlueprintMapLibrary.Map_Find` (`self.BaseStats`) Start) :`BaseValue` Value))
  (`BlueprintMapLibrary.Map_Add` (`self.BaseStats`) (`local.Start`) _structout))

(fn `SetCurrentStatValue`
  (params (Stat :type "/Game/SoulsDeMujerts/Blueprints/Enums/E_Stats Enum" :default "NewEnumerator0") (Value :type "Float (double-precision)"))
  (`BlueprintMapLibrary.Map_Add` (`self.CurrentStats`) Stat Value)
  (`self.OnCurrentStatValueUpdate` (`local.Stat`) (`local.Value`)))

(fn `SetMaxStartValue`
  (params (Start :type "/Game/SoulsDeMujerts/Blueprints/Enums/E_Stats Enum" :default "NewEnumerator0") (Value :type "Float (double-precision)"))
  (bind _structout (setmembers `/Game/SoulsDeMujerts/Blueprints/Structs/F_BaseStat` :`StructRef` (`BlueprintMapLibrary.Map_Find` (`self.BaseStats`) Start) :`MaxValue` Value))
  (`BlueprintMapLibrary.Map_Add` (`self.BaseStats`) (`local.Start`) _structout))

(fn `TakeDamage`
  (params (`In Damage` :type "Float (double-precision)"))
  (`BlueprintMapLibrary.Map_Add` (`self.CurrentStats`) "NewEnumerator1" (`KismetMathLibrary.FMax` (- (`self.Get Current Start Value` "NewEnumerator1") `In Damage`)))
  (if (<= (`self.Get Current Start Value` "NewEnumerator1") 0.0)
    (`/Game/SoulsDeMujerts/Blueprints/Components/StateManagerComponent.Set State` (`Actor.GetComponentByClass` (`self.GetOwner`) "/Game/SoulsDeMujerts/Blueprints/Components/StateManagerComponent.StateManagerComponent_C") "NewEnumerator4")))