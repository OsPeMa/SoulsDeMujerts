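; Base interactable door that opens on interaction, leaving the actual motion to child Blueprints.
; Interact runs only while IsClosed is false, then sets it true despite the name, so the door opens once with no closing logic.
; A dot product against the root's forward vector records the instigator's side in IsSideA.
; The DoorAnimTime timeline feeds DeltaX into the empty OpenUpdate event.
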(event `/Game/SoulsDeMujerts/Blueprints/Interfaces/BP_Interactable.Interact`
  (params (Instigator :type "Actor Object Reference"))
  (if (not (`self.bIsClosed`))
    (set `self.bIsSideA` (`self.Get Side` Instigator))
    (set `self.bIsClosed` true)
    (`self.OpenDoor`)))

(event `OpenDoor`
  (bind (_direction _deltax) (`Timeline|DoorAnimTime`)
    (:`Update`
      (`self.OpenUpdate` _deltax))))

(event `OpenUpdate`
  (params (DeltaX :type "Float (single-precision)")))

(fn `Get Side`
  (params (Character :type "Actor Object Reference"))
  (returns (ReturnValue :type Boolean))
  (return (> 0.0 (`KismetMathLibrary.Dot_VectorVector` (- (`self.K2_GetActorLocation` Character) (`self.K2_GetActorLocation`)) (`SceneComponent.GetForwardVector` (`self.DefaultSceneRoot`))))))

(fn `UserConstructionScript`
  (`parent.UserConstructionScript`))