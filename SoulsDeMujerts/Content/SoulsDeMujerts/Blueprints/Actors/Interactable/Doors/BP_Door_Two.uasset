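; BP_Door_Two is an interactable double door that swings both leaves open according to the side flagged by IsSideA.
; Its OpenUpdate event receives an alpha and lerps SMDoorA and SMDoorB toward their A-side or B-side target rotations.
; Door B starts from a half-turn yaw whose sign flips with the side, while Door A starts from zero.
; The construction script only calls the parent's.
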(event `self.OpenUpdate`
  (params (DeltaX :type "Float (single-precision)"))
  (bind _bissidea (`self.bIsSideA`))
  (`SceneComponent.K2_SetRelativeRotation` (`self.SM_DoorA`) (`KismetMathLibrary.RLerp` (struct) (`KismetMathLibrary.SelectRotator` (`self.DoorARotation_ASide`) (`self.DoorARotation_BSide`) (`self.bIsSideA`)) DeltaX) false false)
  (`SceneComponent.K2_SetRelativeRotation` (`self.SM_DoorB`) (`KismetMathLibrary.RLerp` (`KismetMathLibrary.MakeRotator` 0.0 0.0 (`KismetMathLibrary.SelectFloat` 180.0 -180.0 _bissidea)) (`KismetMathLibrary.SelectRotator` (`self.DoorBRotation_ASide`) (`self.DoorBRotation_BSide`) _bissidea) DeltaX) false false))

(fn `UserConstructionScript`
  (`parent.UserConstructionScript`))