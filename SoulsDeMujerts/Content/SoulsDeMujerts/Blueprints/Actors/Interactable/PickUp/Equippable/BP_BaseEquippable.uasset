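; Base actor for equippable items, providing shared equip state, mesh selection and attachment to the third-person character.
; Equipping sets the equipped flag and snaps the item to a named socket on the instigator's character mesh.
; Unequipping only clears the flag, with no detachment here.
; GetItemMesh returns the static mesh component when it has a mesh assigned, otherwise the skeletal one.
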(fn `Attach Actor`
  (params (SocketName :type Name) (Object :type "Object Object Reference"))
  (`self.K2_AttachToComponent` (`Character.Mesh` (cast `/Game/SoulsDeMujerts/Blueprints/BP_ThirdPersonCharacter` Object :!pure true)) SocketName "SnapToTarget" "SnapToTarget" "SnapToTarget"))

(fn `GetItemMesh`
  (returns (ReturnValue :type "PrimitiveComponent Object Reference"))
  (`/Engine/EditorBlueprintResources/StandardMacros.IsValid` (`StaticMeshComponent.StaticMesh` (`self.itemStaticMesh`))
    (:`Is Valid`
      (return (`self.itemStaticMesh`)))
    (:`Is Not Valid`
      (return (`self.itemSkeletalMesh`)))))

(fn `IsEquipped?`
  (returns (`Return Value` :type Boolean))
  (return (`self.bIsEquipped?`)))

(fn `OnEquipped`
  (params (Instigator :type "Actor Object Reference"))
  (set `self.bIsEquipped?` true)
  (`self.Attach Actor` (`self.Attach Socket Name`) Instigator))

(fn `OnUnequipped`
  (if (`self.bIsEquipped?`)
    (set `self.bIsEquipped?` false)))

(fn `SetIsEquipped`
  (params (`IsEquipped?` :type Boolean))
  (set `self.bIsEquipped?` `IsEquipped?`))

(fn `UserConstructionScript`)