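; BP_BaseWeapon is the base equippable weapon actor, handling attachment to a character and registration with its combat system.
; On equip it attaches to the hand or holstered socket depending on whether combat is enabled, becomes the CombatComponent's main weapon and sends its combat type to the AnimInstance.
; Its CollisionComponent takes the item mesh, ignores the wielder and owner, and currently only prints the hit actor's name on hit.
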(event `self.CollisionComponent.OnHit`
  (params (HitResult :type "HitResult Structure"))
  (`KismetSystemLibrary.PrintString` (`KismetSystemLibrary.GetDisplayName` (`.HitActor` (`GameplayStatics.BreakHitResult` HitResult)))))

(fn `OnEquipped`
  (params (Instigator :type "Actor Object Reference"))
  (`/Game/SoulsDeMujerts/Blueprints/Components/CollisionComponent.AddActorToIgnore` (`self.CollisionComponent`) Instigator)
  (set `self.CombatComponent` (`self.GetComponentByClass` Instigator "/Game/SoulsDeMujerts/Blueprints/Components/CombatComponent.CombatComponent_C"))
  (`self.Attach Actor` (select `bool` (`/Game/SoulsDeMujerts/Blueprints/Components/CombatComponent.IsCombatEnabled?` (`self.CombatComponent`)) :`false` (`self.Attach Socket Name`) :`true` (`self.HandSocketName`)) Instigator)
  (`/Game/SoulsDeMujerts/Blueprints/Components/CombatComponent.SetMainWeapon` (`self.CombatComponent`) self)
  (message `/Game/SoulsDeMujerts/Blueprints/Interfaces/BPI_AnimationInstance.UpdateCombatType` (`SkeletalMeshComponent.GetAnimInstance` (`Character.Mesh` (cast `Character` Instigator :!pure true))) (`self.CombatType`))
  (`/Game/SoulsDeMujerts/Blueprints/Components/CollisionComponent.SetCollisionMesh` (`self.CollisionComponent`) (`self.GetItemMesh`))
  (`/Game/SoulsDeMujerts/Blueprints/Components/CollisionComponent.AddActorToIgnore` (`self.CollisionComponent`) (`self.GetOwner`)))

(fn `UserConstructionScript`
  (`parent.UserConstructionScript`))